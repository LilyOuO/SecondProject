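; Game controller for an aim-and-charge shooting game that creates the game UI and finds the arrow actor on BeginPlay.
; The start event plays a timeline that sweeps the shot angle and rotates the arrow's yaw to match.
; The charge event plays a second timeline that drives the UI progress bar and shot power.
; Separate events add or subtract score; the shot itself is not fired here.
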(event `self.ReceiveBeginPlay`
  (`KismetSystemLibrary.PrintString` "GameController 開始載入")
  ; 建立遊戲 UI
  (bind _returnvalue (`|CreateWidget` "/Game/Class_B/WBP_GameUI_B.WBP_GameUI_B_C"))
  (set `self.遊戲介面` _returnvalue)
  (`UserWidget.AddToViewport` _returnvalue 0)
  ; 取得箭頭物件
  (bind _returnvalue_2 (`GameplayStatics.GetActorOfClass` "/Game/Class_B/BP_箭頭方向_B.BP_箭頭方向_B_C"))
  (set `self.箭頭物件` _returnvalue_2)
  (set `self.射擊力量` 10.0))

(event `OnStartButtonClick`
  ; 自定義的開始事件
  (`KismetSystemLibrary.PrintString` "開始事件被觸發")
  (bind (_direction _newtrack_0) (`Timeline|Timeline`)
    (:`Update`
      (bind _output_get (set `self.射擊角度` (`KismetMathLibrary.Lerp` -60.0 60.0 _newtrack_0)))
      (`self.K2_SetActorRotation` (`self.箭頭物件`) (`KismetMathLibrary.MakeRotator` 0.0 0.0 _output_get) false))))

(event `觸發蓄力事件`
  ; 蓄力事件相關內容
  ;; 蓄力事件
  (`KismetSystemLibrary.PrintString` "蓄力事件被觸發")
  (bind (_direction `_newtrack_蓄力`) (`Timeline|Timeline_蓄力`)
    (:`Update`
      (`ProgressBar.SetPercent` (`/Game/Class_B/WBP_GameUI_B.ProgressBar_0` (`self.遊戲介面`)) `_newtrack_蓄力`)
      (set `self.射擊力量` (`KismetMathLibrary.Lerp` 10.0 100.0 `_newtrack_蓄力`)))))

(event `碰到得分區事件`
  ; 分數 = 分數 + 1
  (set `self.分數` (+ (`self.分數`) 1)))

(event `扣分事件`
  ; 分數 = 分數 - 1
  (set `self.分數` (- (`self.分數`) 1)))

(fn `UserConstructionScript`)