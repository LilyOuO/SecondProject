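; Demo game controller that sets up the game UI, drives the shot direction indicator and keeps the score.
; BeginPlay adds the UI widget to the viewport and caches the direction indicator actor found in the level.
; A rotation button event plays a timeline that lerps the shot direction across a yaw arc and applies it to that indicator.
; A score-area touch event increments Score.
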(event `self.ReceiveBeginPlay`
  (`KismetSystemLibrary.PrintString` "GameController 開始載入")
  ; 把 UI 新建出來
  (bind _returnvalue (`|CreateWidget` "/Game/InClassDemo/FirstProject/WBP_GameUI_Demo.WBP_GameUI_Demo_C"))
  (`UserWidget.AddToViewport` _returnvalue 0)
  (bind _returnvalue_2 (`GameplayStatics.GetActorOfClass` "/Game/InClassDemo/FirstProject/BP_方向指示_Demo.BP_方向指示_Demo_C"))
  (set `self.方向物件` _returnvalue_2))

(event `OnRotationButtonClick`
  (`KismetSystemLibrary.PrintString` "旋轉事件觸發")
  (bind (_direction _rotationtrack) (`Timeline|RotationTimeline`)
    (:`Update`
      (bind _output_get (set `self.射出方向` (`KismetMathLibrary.Lerp` 60.0 -60.0 _rotationtrack)))
      (`self.K2_SetActorRotation` (`self.方向物件`) (`KismetMathLibrary.MakeRotator` 0.0 0.0 _output_get) false))))

(event `TouchScoreArea`
  (`KismetSystemLibrary.PrintString` "碰到得分區")
  (set `self.Score` (+ (`self.Score`) 1)))

(fn `UserConstructionScript`)